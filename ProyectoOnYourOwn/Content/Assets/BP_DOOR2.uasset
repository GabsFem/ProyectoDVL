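; BP_DOOR2 is a door Blueprint that slides the DOOR component up on overlap and back down afterwards.
; Begin overlap on RE plays the DOORMOVEMENT timeline, while end overlap on DOOR itself, not RE, plays a separate Timeline_0 in reverse from its end.
; Both timelines lerp from the door's current relative location toward the raised position or zero, so the motion compounds each update rather than following the curve directly.
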(event OnComponentBeginOverlap(RE)
  (params (OverlappedComponent :type Primitive%20Component%20Object%20Reference) (OtherActor :type Actor%20Object%20Reference) (OtherComp :type Primitive%20Component%20Object%20Reference) (OtherBodyIndex :type Integer) (bFromSweep :type Boolean) (SweepResult :type Hit%20Result%20Structure%20%28by%20ref%29))
  ;[1 1 1] OPEN DOOR
  (bind _door (Timeline|DOORMOVEMENT PlayFromStart)
    (:Update
      (Transformation|SetRelativeLocation (Variables|Default|GetDOOR) (Math|Vector|Lerp(Vector) (Variables|/Script/Engine.SceneComponent|GetRelativeLocation (Variables|Default|GetDOOR)) "0, 0,243.000000" _door) false false))))

(event OnComponentEndOverlap(DOOR)
  (params (OverlappedComponent :type Primitive%20Component%20Object%20Reference) (OtherActor :type Actor%20Object%20Reference) (OtherComp :type Primitive%20Component%20Object%20Reference) (OtherBodyIndex :type Integer))
  ;[1 1 1] CLOSE DOOR
  (bind _door (Timeline|Timeline_0 ReverseFromEnd)
    (:Update
      (Transformation|SetRelativeLocation (Variables|Default|GetDOOR) (Math|Vector|Lerp(Vector) (Variables|/Script/Engine.SceneComponent|GetRelativeLocation (Variables|Default|GetDOOR)) "0, 0, 0" _door) false false))))

(event EventBeginPlay)

(event Collision|EventActorBeginOverlap
  (params (OtherActor :type Actor%20Object%20Reference)))

(event EventTick
  (params (DeltaSeconds :type Float%20%28single-precision%29)))

(fn ConstructionScript)